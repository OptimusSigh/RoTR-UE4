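; Base class for buff abilities, which plays a cast montage, registers with the HUD buff panel and lasts for a set lifespan.
; On begin play it destroys same-class actors attached to the caster and starts the montage.
; Casting sets the lifespan, applies the buff, starts a non-looping tick timer and triggers the effect from a montage notify.
; TickBuff and ClearBuff are empty stubs, and EndPlay signals the buff's removal.
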(event Custom|TickBuff)

(event EventBeginPlay
  (CallFunction|ClearDuplicates)
  (|CallParentFunction)
  (Animation|Montage|PlayMontage (Variables|/Script/Engine.Character|GetMesh (Variables|Default|GetPlayerReference)) "/Game/Art_Assets/Animations/Monk/Monk_Cast.Monk_Cast"))

(event EventEndPlay
  (params (EndPlayReason :type EEndPlayReason%20Enum :default "Destroyed"))
  (Default|CallBuffRemoved))

(event EventCastAbility
  (Actor|SetLifeSpan (Variables|Default|GetBuffTimer))
  (CallFunction|ApplyBuff)
  (bind _returnvalue (Utilities|Time|SetTimerbyEvent (delegate Custom|TickBuff) (Variables|Default|GetBuffTickRate)))
  (Variables|Default|SetBuffTickTimer _returnvalue)
  (Animation|Montage|PlayMontage (Variables|/Script/Engine.Character|GetMesh (Variables|Default|GetPlayerReference)) "/Game/Art_Assets/Animations/Monk/Monk_Cast.Monk_Cast" 1.0 0.0 "CastEnd"
    (:OnNotifyBegin
      (CallFunction|ActivateEffect))))

(fn ConstructionScript
  (|CallParentFunction))

(fn ApplyBuff
  (Default|AddBufftoUI (Variables|/Game/BluePrints/UI/HUD_UI.HUD_UI_C|GetBuffPanel_UI (Variables|Default|GetHUD_UI)) self))

(fn ClearBuff)

(fn ClearDuplicates
  (for _array_element (Actor|GetAttachedActors (Variables|Default|GetCaster) false)
    (if (== (Utilities|GetClass _array_element) (Utilities|GetClass self))
      (Actor|DestroyActor _array_element))))