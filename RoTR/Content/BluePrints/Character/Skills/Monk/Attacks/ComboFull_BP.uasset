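; Monk attack skill Blueprint that plays a full combo of six kick and punch montages on the player's mesh.
; BeginPlay runs the parent logic, then plays the montage selected by ComboCount modulo six at slightly increased speed.
; Each completed montage increments ComboCount and starts the next, cycling with no exit condition or input check in this graph.
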(event EventBeginPlay
  (|CallParentFunction)
  (Animation|Montage|PlayMontage (Variables|/Script/Engine.Character|GetMesh (Variables|Default|GetPlayerReference)) (Utilities|Select :Index (Math|Integer|%(Integer) (Variables|Default|GetComboCount) 6) :Option%200 "/Game/Art_Assets/Animations/Monk/Double_Kick_Montage.Double_Kick_Montage" :Option%201 "/Game/Art_Assets/Animations/Monk/Flurry_Of_Punches_Montage.Flurry_Of_Punches_Montage" :Option%202 "/Game/Art_Assets/Animations/Monk/FlyingKick_Montage.FlyingKick_Montage" :Option%203 "/Game/Art_Assets/Animations/Monk/Kick_Left1_Montage.Kick_Left1_Montage" :Option%204 "/Game/Art_Assets/Animations/Monk/Punch_Right1_Montage.Punch_Right1_Montage" :Option%205 "/Game/Art_Assets/Animations/Monk/Punch_Left1_Montage.Punch_Left1_Montage") 1.1 :!label _label
    (:OnCompleted
      (Math|Integer|IncrementInt (Variables|Default|GetComboCount)
        (:%20%20
          (goto _label))))))

(fn ConstructionScript
  (|CallParentFunction))