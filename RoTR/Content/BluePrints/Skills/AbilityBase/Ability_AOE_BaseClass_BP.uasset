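; Base class for area-of-effect abilities, extending a parent ability class to place a particle effect on the ground under the player.
; BeginPlay starts the area-attack montage on the player's mesh, and CastAbility replays it from the CastEnd section.
; A montage notify calls ActivateEffect, which activates the particles, zeroes rotation and moves the actor to the hit of a debug-drawn downward trace, without checking for a hit.
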(event EventCastAbility
  (|CallParentFunction)
  (Animation|Montage|PlayMontage (Variables|/Script/Engine.Character|GetMesh (Variables|Default|GetPlayerReference)) "/Game/Art_Assets/Animations/Monk/StandingMagicAreaAttack_Montage.StandingMagicAreaAttack_Montage" 1.0 0.0 "CastEnd"
    (:OnNotifyBegin
      (CallFunction|ActivateEffect))))

(event EventActivateEffect
  (bind _returnvalue (Game|GetPlayerCharacter 0))
  (bind _returnvalue_2 (Transformation|GetActorLocation _returnvalue))
  (|CallParentFunction)
  (Components|Activation|Activate (Variables|Default|GetParticleSystem) false)
  (Transformation|SetActorRotation "0, 0, 0")
  (bind _outhit (Collision|LineTraceByChannel _returnvalue_2 (+ _returnvalue_2 "0, 0,-1000.000000") "TraceTypeQuery1" false (Utilities|Array|MakeArray _returnvalue) "ForDuration"))
  (Transformation|SetActorLocation (.location _outhit) false false))

(event EventBeginPlay
  (|CallParentFunction)
  (Animation|Montage|PlayMontage (Variables|/Script/Engine.Character|GetMesh (Variables|Default|GetPlayerReference)) "/Game/Art_Assets/Animations/Monk/StandingMagicAreaAttack_Montage.StandingMagicAreaAttack_Montage"))

(fn ConstructionScript
  (|CallParentFunction))