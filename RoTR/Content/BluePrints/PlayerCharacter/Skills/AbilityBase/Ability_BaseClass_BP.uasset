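; Base Blueprint for player skill abilities, handling cast time, interruption and release of an ability actor.
; On BeginPlay it attaches to the caster's mesh, then either shows a HUD cast bar with a success binding or casts immediately.
; Tick requests interruption through the player when interruptible and movement input is detected.
; CastAbility only detaches the actor, InterruptCast destroys it, and ActivateEffect is an empty stub.
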(event EventBeginPlay
  (Transformation|AttachComponentToComponent (Variables|/Script/Engine.Character|GetMesh (Variables|Default|GetCaster)) "None" "KeepRelative" "KeepRelative" "KeepRelative" true)
  (bind _asro_trplayer_bp (Utilities|Casting|CastToRoTRPlayer_BP (Game|GetPlayerCharacter 0)))
  (Variables|Default|SetPlayerReference _asro_trplayer_bp)
  (bind _returnvalue (Actor|GetActorOfClass "/Game/BluePrints/GameManager_BP.GameManager_BP_C"))
  (Variables|Default|SetHUD_UI (Variables|/Game/BluePrints/GameManager_BP.GameManager_BP_C|GetHUD _returnvalue))
  (CallFunction|BiginCasting))

(event EventTick
  (params (DeltaSeconds :type Float%20%28single-precision%29))
  (bind _playerreference (Variables|Default|GetPlayerReference))
  (if (.isinteruptable (Variables|Default|GetAbilityDetails))
    (if (or (!= (Variables|/Game/BluePrints/PlayerCharacter/Player/RoTRPlayer_BP.RoTRPlayer_BP_C|GetMoveForwardValueRef _playerreference) 0.0) (!= (Variables|/Game/BluePrints/PlayerCharacter/Player/RoTRPlayer_BP.RoTRPlayer_BP_C|GetMoveRightValueRef _playerreference) 0.0))
      (Default|CallInterruptCasting _playerreference))))

(fn ConstructionScript)

(fn BiginCasting
  (if (> (.casttime (Variables|Default|GetAbilityDetails)) 0.0)
    (bind _castbarreference (Default|DisplayCastBar (Variables|Default|GetHUD_UI) self))
    (EventDispatchers|BindEventtoCastSucsessful _castbarreference (EventDispatchers|CreateEvent :!event CastAbility))
    (else
      (CallFunction|CastAbility))))

(fn CastAbility
  (Transformation|DetachFromActor "KeepWorld" "KeepWorld" "KeepWorld"))

(fn InterruptCast
  (Actor|DestroyActor))

(fn ActivateEffect)