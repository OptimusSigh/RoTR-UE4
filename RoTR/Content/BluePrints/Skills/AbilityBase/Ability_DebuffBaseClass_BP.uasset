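; Base ability class for debuff skills, which attach themselves as actors to the player's current target.
; Plays a spell-casting montage on spawn, jumping to its end section on cast.
; Casting destroys same-class duplicates on the target (or itself without a valid target), sets a lifespan, attaches and refreshes the target UI.
; A looping timer fires an empty tick event at the debuff tick rate.
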(event Custom|Dubuff%20Tick)

(event EventBeginPlay
  (|CallParentFunction)
  (Animation|Montage|PlayMontage (Variables|/Script/Engine.Character|GetMesh (Variables|Default|GetPlayerReference)) "/Game/Art_Assets/Animations/Monk/WideArmSpellCasting_Montage.WideArmSpellCasting_Montage"))

(event EventCastAbility
  (|CallParentFunction)
  (CallFunction|ClearDuplicates)
  (Actor|SetLifeSpan (Variables|Default|GetDebuffLifeSpan))
  (CallFunction|ApplyDebuff)
  (bind _returnvalue (Utilities|Time|SetTimerbyEvent (delegate Custom|Dubuff%20Tick) (Variables|Default|GetDebuffTickRate) true))
  (Variables|Default|SetDebuffTickTimer _returnvalue)
  (Animation|Montage|PlayMontage (Variables|/Script/Engine.Character|GetMesh (Variables|Default|GetPlayerReference)) "/Game/Art_Assets/Animations/Monk/WideArmSpellCasting_Montage.WideArmSpellCasting_Montage" 1.0 0.0 "CastEnd"))

(fn ConstructionScript
  (|CallParentFunction))

(fn ClearDuplicates
  (bind _self self)
  (bind _currenttarget (Variables|/Game/BluePrints/PlayerCharacter/Player/RoTRPlayer_BP.RoTRPlayer_BP_C|GetCurrentTarget (Variables|Default|GetPlayerReference))
    (:then
      (for _array_element (Actor|GetAttachedActors _currenttarget false)
        (if (and (== (Utilities|GetClass _array_element) (Utilities|GetClass _self)) (!= _array_element _self))
          (Actor|DestroyActor _array_element))))
    (:else
      (Actor|DestroyActor))))

(fn ApplyDebuff
  (bind _asro_trplayer_bp (Utilities|Casting|CastToRoTRPlayer_BP (Game|GetPlayerCharacter 0)))
  (Transformation|AttachActorToActor (Variables|/Game/BluePrints/PlayerCharacter/Player/RoTRPlayer_BP.RoTRPlayer_BP_C|GetCurrentTarget _asro_trplayer_bp) "None" "SnapToTarget" "SnapToTarget" "SnapToTarget" true)
  (Default|UpdateTargetUI (Variables|/Game/BluePrints/UI/HUD/Player_HUD_UI.Player_HUD_UI_C|GetTargeted_UI (Variables|Default|GetHUD_UI))))