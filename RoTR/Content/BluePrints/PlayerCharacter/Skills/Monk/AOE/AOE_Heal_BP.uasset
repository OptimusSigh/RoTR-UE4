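; Monk area-of-effect skill actor that applies a periodic heal effect to players standing inside it.
; On activation it runs the parent logic, shows its decal and particle system, sets its lifespan from Duration and starts a looping timer at the DOTTimer interval.
; Each tick gathers RoTRPlayer_BP actors overlapping AbilityRootCollision and passes HealAmount to them through ApplyDamage, so healing uses the damage pipeline.
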(event Custom|TickEffects
  (for _array_element (Collision|GetOverlappingActors (Variables|Default|GetAbilityRootCollision) "/Game/BluePrints/PlayerCharacter/Player/RoTRPlayer_BP.RoTRPlayer_BP_C" :!class /Script/Engine.PrimitiveComponent)
    (Game|Damage|ApplyDamage _array_element (Variables|Default|GetHealAmount) 0 0)))

(event EventActivateEffect
  (|CallParentFunction)
  (Rendering|SetVisibility (Variables|Default|GetDecal) true false)
  (Rendering|SetVisibility (Variables|Default|GetParticleSystem) true false)
  (Actor|SetLifeSpan (Variables|Default|GetDuration))
  (Utilities|Time|SetTimerbyEvent (delegate Custom|TickEffects) (Variables|Default|GetDOTTimer) true))

(fn ConstructionScript
  (|CallParentFunction))