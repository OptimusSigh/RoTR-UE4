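; Base Blueprint class for homing projectile abilities in the skill system.
; On BeginPlay it runs the parent logic, then sets the projectile movement's homing target to the root component of the player's current target.
; Casting, effect activation and construction only call their parent implementations.
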(event EventBeginPlay
  (|CallParentFunction)
  (Variables|/Script/Engine.ProjectileMovementComponent|SetHomingTargetComponent (Variables|Default|GetProjectileMovement) (Variables|/Script/Engine.Actor|GetRootComponent (Variables|/Game/BluePrints/PlayerCharacter/Player/RoTRPlayer_BP.RoTRPlayer_BP_C|GetCurrentTarget (Variables|Default|GetPlayerReference)))))

(event EventCastAbility
  (|CallParentFunction))

(event EventActivateEffect
  (|CallParentFunction))

(fn ConstructionScript
  (|CallParentFunction))