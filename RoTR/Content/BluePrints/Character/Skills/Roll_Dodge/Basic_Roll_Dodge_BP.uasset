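; Roll/dodge skill actor that, on BeginPlay, plays the player's evasive montage and then destroys itself in most branches.
; When locked on, it plays a directional dodge chosen from movement input, defaulting to backwards.
; Otherwise, unless falling or already stepping back, it rolls with input or steps back without.
; Dodges and rolls interrupt other montages but not themselves, while the step back waits for none to be playing.
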(event Custom|Call
  (params (Direction :type DodgeDirections_Enum%20Enum :default "NewEnumerator0"))
  (bind _playerreference (Variables|Default|GetPlayerReference))
  (if (Variables|/Game/BluePrints/Character/Player/RoTRPlayer_BP.RoTRPlayer_BP_C|GetLockedOnATarget _playerreference)
    (CallFunction|PlayHighPriorityMontage (Utilities|Select :Index Direction :NewEnumerator0 "/Game/Art_Assets/Animations/Monk/Monk_Dodge_Backwards_Montage.Monk_Dodge_Backwards_Montage" :NewEnumerator1 "/Game/Art_Assets/Animations/Monk/Monk_Dodge_Left_Montage.Monk_Dodge_Left_Montage" :NewEnumerator2 "/Game/Art_Assets/Animations/Monk/Monk_Dodge_Right_Montage.Monk_Dodge_Right_Montage" :NewEnumerator3 "/Game/Art_Assets/Animations/Monk/Monk_Dodge_Forward_Montage.Monk_Dodge_Forward_Montage") 1.5 "None")
    (Actor|DestroyActor)
    (elif (AI|Components|NavMovement|IsFalling (Variables|/Script/Engine.Character|GetCharacterMovement _playerreference))
      (Actor|DestroyActor)
      (elif (not (Animation|Montage|MontageIsPlaying (Components|SkeletalMesh|GetAnimInstance (Variables|/Script/Engine.Character|GetMesh _playerreference)) "/Game/Art_Assets/Animations/Monk/StepBack_Montage.StepBack_Montage"))
        (if (Utilities|HasPlayerMovment)
          (CallFunction|PlayHighPriorityMontage "/Game/Art_Assets/Animations/Monk/Monk_Roll.Monk_Roll" 1.5 "None")
          (Actor|DestroyActor)
          (else
            (CallFunction|TryPlayMontage "/Game/Art_Assets/Animations/Monk/StepBack_Montage.StepBack_Montage" 1.0 "None")
            (Actor|DestroyActor)))))))

(event EventBeginPlay
  (|CallParentFunction)
  (CallFunction|Call (.ReturnValue (|ChooseDodgeDirection))))

(fn ConstructionScript
  (|CallParentFunction))

(fn PlayHighPriorityMontage
  (params (Montage :type Anim%20Montage%20Object%20Reference) (InPlayRate :type Float%20%28single-precision%29) (StartSectionName :type Name))
  (bind _playerreference (Variables|Default|GetPlayerReference))
  (if (not (Animation|Montage|MontageIsPlaying (Components|SkeletalMesh|GetAnimInstance (Variables|/Script/Engine.Character|GetMesh _playerreference)) Montage))
    (bind _output_get (LocalVariables|SetHighPriorityMontage Montage))
    (Animation|PlayAnimMontage _playerreference _output_get InPlayRate StartSectionName)
    (return 0.0)))

(fn TryPlayMontage
  (params (Montage :type Anim%20Montage%20Object%20Reference) (InPlayRate :type Float%20%28single-precision%29) (StartSectionName :type Name))
  (bind _playerreference (Variables|Default|GetPlayerReference))
  (if (not (Animation|Montage|MontageIsPlaying (Components|SkeletalMesh|GetAnimInstance (Variables|/Script/Engine.Character|GetMesh _playerreference)) 0))
    (Animation|PlayAnimMontage _playerreference Montage InPlayRate StartSectionName)
    (return 0.0)))