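; TestDummy_BP is an NPC test dummy that takes damage and has a health bar widget.
; On BeginPlay it casts the HealthBar component's widget to EnemyHealthBar_BP and passes itself as EnemyBP.
; TakeDamage subtracts damage from Health, clamped between zero and its current value, then sets HealthPercent assuming a maximum of 100.
; It has no death handling.
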(event EventBeginPlay
  (bind _asenemy_health_bar_bp (Utilities|Casting|CastToEnemyHealthBar_BP (UserInterface|GetUserWidgetObject (Variables|Default|GetHealthBar))))
  (Variables|/Game/BluePrints/UI/EnemyHealthBar_BP.EnemyHealthBar_BP_C|SetEnemy_BP _asenemy_health_bar_bp self))

(fn ConstructionScript)

(fn TakeDamage
  (params (Damage :type Float%20%28single-precision%29))
  (bind _output_get (Variables|Default|SetHealth (Math|Float|Clamp(Float) (- (Variables|Default|GetHealth) Damage) 0.0 (Variables|Default|GetHealth))))
  (Variables|Default|SetHealthPercent (/ _output_get 1e+02)))