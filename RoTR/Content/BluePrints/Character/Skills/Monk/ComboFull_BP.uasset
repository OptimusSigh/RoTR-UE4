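; Monk skill Blueprint that plays a looping six-attack combo of punch, palm and kick animations on the player.
; On BeginPlay it runs the parent logic, then plays a montage on the player's mesh, selected by the combo count modulo six.
; Each completed montage increments the count and starts the next at slightly raised speed, with no stop condition in this graph.
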(event EventBeginPlay
  (|CallParentFunction)
  (Animation|Montage|PlayMontage (Variables|/Script/Engine.Character|GetMesh (Variables|Default|GetPlayerReference)) (Utilities|Select :Index (Math|Integer|%(Integer) (Variables|Default|GetComboCount) 6) :Option%200 "/Game/Art_Assets/Animations/Monk/Monk_Right_Punch_Montage.Monk_Right_Punch_Montage" :Option%201 "/Game/Art_Assets/Animations/Monk/Monk_Standing_Melee_Punch_Montage.Monk_Standing_Melee_Punch_Montage" :Option%202 "/Game/Art_Assets/Animations/Monk/Monk_Left_Palm_Montage.Monk_Left_Palm_Montage" :Option%203 "/Game/Art_Assets/Animations/Monk/Monk_Right_Kick_Montage.Monk_Right_Kick_Montage" :Option%204 "/Game/Art_Assets/Animations/Monk/Flurry_Of_Punches_Montage.Flurry_Of_Punches_Montage" :Option%205 "/Game/Art_Assets/Animations/Monk/Flying_Kick_Montage.Flying_Kick_Montage") 1.1 :!label _label
    (:OnCompleted
      (Math|Integer|IncrementInt (Variables|Default|GetComboCount)
        (:%20%20
          (goto _label))))))

(fn ConstructionScript
  (|CallParentFunction))