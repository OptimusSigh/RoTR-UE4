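; Enemy NPC Blueprint that can be targeted by lock-on and takes damage with on-screen feedback.
; TargetLockON toggles a target marker through a FlipFlop.
; AnyDamage plays a head-hit animation and applies damage only while the mesh is not already animating, so hits during playback are ignored.
; TakeDamage spawns a screen-projected combat number widget and updates health and its percentage; a helper returns distance to the player.
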(event Game|Damage|EventAnyDamage
  (params (Damage :type Float%20%28single-precision%29) (DamageType :type Damage%20Type%20Object%20Reference) (InstigatedBy :type Controller%20Object%20Reference) (DamageCauser :type Actor%20Object%20Reference))
  (if (not (Audio|Components|Audio|IsPlaying (Variables|Character|GetMesh)))
    (Components|Animation|PlayAnimation (Variables|Character|GetMesh) "/Game/Art_Assets/Animations/Head_Hit.Head_Hit" false)
    (Development|PrintString (Utilities|String|ToString(Float) Damage))
    (CallFunction|TakeDamage Damage)))

(event EventTargetLockON
  (bind _targetvisual (Variables|Default|GetTargetVisual))
  (Utilities|FlowControl|FlipFlop
    (:A
      (Development|SetHiddeninGame _targetvisual false false))
    (:B
      (Development|SetHiddeninGame _targetvisual true false))))

(fn ConstructionScript)

(fn TakeDamage
  (params (Damage :type Float%20%28single-precision%29))
  (CallFunction|ShowCombatText (Transformation|GetActorLocation) Damage)
  (bind _output_get (Variables|Default|SetHealth (Math|Float|Clamp(Float) (- (Variables|Default|GetHealth) Damage) 0.0 (Variables|Default|GetHealth))))
  (Variables|Default|SetHealthPercent (/ _output_get 1e+02)))

(fn ShowCombatText
  (params (WorldLocation :type Vector) (Damage :type Float%20%28single-precision%29))
  ;[1 1 1] Combat Text
  (bind _returnvalue (UserInterface|CreateWidget :Class "/Game/BluePrints/UI/CombatText/CombatNumbers.CombatNumbers_C" :StartScreenLocation (.ScreenPosition (Class|GameplayStatics|ProjectWorldtoScreen (Game|GetPlayerController 0) WorldLocation false)) :DamageToDisplay Damage))
  (UserInterface|Viewport|AddtoViewport _returnvalue 0))

(fn DistancefromPlayerCheck
  (return (Transformation|GetDistanceTo (Game|GetPlayerCharacter 0))))