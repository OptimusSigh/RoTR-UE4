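; Base Blueprint for projectile abilities that a character casts from the hand.
; On BeginPlay it plays the casting montage on the player mesh, then attaches to the caster's right-hand socket.
; CastAbility plays the montage's CastEnd section, and its notify calls ActivateEffect, which activates the projectile movement component to launch the projectile.
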(event EventBeginPlay
  (|CallParentFunction)
  (Animation|Montage|PlayMontage (Variables|/Script/Engine.Character|GetMesh (Variables|Default|GetPlayerReference)) "/Game/Art_Assets/Animations/Monk/CastingSpell_Montage.CastingSpell_Montage"
    (:then
      (Transformation|AttachComponentToComponent (Variables|/Script/Engine.Character|GetMesh (Variables|Default|GetCaster)) "hand_r" "SnapToTarget" "SnapToTarget" "SnapToTarget" true))))

(event EventActivateEffect
  (|CallParentFunction)
  (Components|Activation|Activate (Variables|Default|GetProjectileMovement) false))

(event EventCastAbility
  (|CallParentFunction)
  (Animation|Montage|PlayMontage (Variables|/Script/Engine.Character|GetMesh (Variables|Default|GetPlayerReference)) "/Game/Art_Assets/Animations/Monk/CastingSpell_Montage.CastingSpell_Montage" 1.0 0.0 "CastEnd"
    (:OnNotifyBegin
      (CallFunction|ActivateEffect))))

(fn ConstructionScript
  (|CallParentFunction))