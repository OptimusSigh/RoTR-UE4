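; Base enemy NPC Blueprint that handles health, hit reactions, knockout and floating damage numbers.
; On BeginPlay it fills health and hands itself to its health bar widget.
; AnyDamage is ignored while the mesh is animating; otherwise it plays a head hit, lowers clamped health and spawns a combat number widget at the enemy's projected screen position.
; At zero health it plays the knockout animation and destroys the health bar.
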(event Game|Damage|EventAnyDamage
  (params (Damage :type Float%20%28single-precision%29) (DamageType :type Damage%20Type%20Object%20Reference) (InstigatedBy :type Controller%20Object%20Reference) (DamageCauser :type Actor%20Object%20Reference))
  (if (not (Audio|Components|Audio|IsPlaying (Variables|Character|GetMesh)))
    (Components|Animation|PlayAnimation (Variables|Character|GetMesh) "/Game/Art_Assets/Animations/ConvertedMixamo/HeadHit.HeadHit" false)
    (CallFunction|TakeDamage Damage)
    (if (== (Variables|Default|GetHealthCurrent) 0.0)
      (Components|Animation|PlayAnimation (Variables|Character|GetMesh) "/Game/Art_Assets/Animations/ConvertedMixamo/KnockedOut.KnockedOut" false)
      (Components|DestroyComponent (Variables|Default|GetHealthBar)))))

(event EventBeginPlay
  (Variables|Default|SetHealthCurrent (Variables|Default|GetHealthMax))
  (bind _asenemy_health_bar_ui (Utilities|Casting|CastToEnemyHealthBar_UI (UserInterface|GetUserWidgetObject (Variables|Default|GetHealthBar))))
  (Variables|/Game/BluePrints/UI/HealthBars/EnemyHealthBar_UI.EnemyHealthBar_UI_C|SetEnemy_BP _asenemy_health_bar_ui self))

(fn ConstructionScript)

(fn TakeDamage
  (params (Damage :type Float%20%28single-precision%29))
  (CallFunction|ShowCombatText (Transformation|GetActorLocation) Damage)
  (Variables|Default|SetHealthCurrent (Math|Float|Clamp(Float) (- (Variables|Default|GetHealthCurrent) Damage) 0.0 (Variables|Default|GetHealthCurrent)))
  (Variables|Default|SetHealthPercent (/ (Variables|Default|GetHealthCurrent) (Variables|Default|GetHealthMax))))

(fn ShowCombatText
  (params (WorldLocation :type Vector) (Damage :type Float%20%28single-precision%29))
  ;[1 1 1] Combat Text
  (bind _returnvalue (UserInterface|CreateWidget :Class "/Game/BluePrints/UI/CombatText/CombatNumbers_UI.CombatNumbers_UI_C" :StartScreenLocation (.ScreenPosition (Class|GameplayStatics|ProjectWorldtoScreen (Game|GetPlayerController 0) WorldLocation false)) :DamageToDisplay Damage))
  (UserInterface|Viewport|AddtoViewport _returnvalue 0))