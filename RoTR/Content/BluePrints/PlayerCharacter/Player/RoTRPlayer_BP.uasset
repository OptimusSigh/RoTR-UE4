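; Player character Blueprint handling basic attack, block, target lock-on, emotes, mouse release and a debug position save/load.
; Basic attack spawns a combo actor behind a DoOnce, which the cancel input resets while destroying that actor and playing a block montage.
; Targeting sphere-traces for interface implementers, locks onto the first, and Tick turns character and camera toward it.
; The held radial emote wheel picks montages on left click, briefly disabling movement.
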(event Custom|UnlockComboEvent
  (bind _returnvalue (Game|GetPlayerCharacter 0))
  (Utilities|FlowControl|DoOnce false) ; enters at Reset
)

(event EventTick
  (params (DeltaSeconds :type Float%20%28single-precision%29))
  ;[1 1 1] Tick
  (CallFunction|LookatTarget)
  (Variables|Default|SetMoveForwardValueRef (Input|AxisValues|GetMoveForward))
  (Variables|Default|SetMoveRightValueRef (Input|AxisValues|GetMoveRight)))

(event Input|ActionEvents|InputActionEmote
  (params (Key :type Key%20Structure :default "None"))
  (bind _returnvalue (Game|GetPlayerController 0))
  ;[1 1 1] Emoting
  (:Pressed
    (Variables|Default|SetIsEmoteWheelOpen true)
    (bind _returnvalue_2 (UserInterface|CreateWidget "/Game/BluePrints/UI/RadialMenu/EmoteRadialMenu_UI.EmoteRadialMenu_UI_C"))
    (bind _output_get (Variables|Default|SetEmoteWheelRef _returnvalue_2))
    (Default|StartEmoteSelection _output_get)
    (UserInterface|Viewport|AddtoViewport _output_get 0)
    (Variables|/Script/Engine.PlayerController|SetbShowMouseCursor _returnvalue true)
    (Input|SetIgnoreLookInput _returnvalue true)
    (Input|SetInputModeGameandUI _returnvalue (Variables|Default|GetEmoteWheelRef) "DoNotLock" false))
  (:Released
    (Variables|Default|SetIsEmoteWheelOpen false)
    (Widget|RemovefromParent (Variables|Default|GetEmoteWheelRef))
    (Variables|/Script/Engine.PlayerController|SetbShowMouseCursor _returnvalue false)
    (Input|SetIgnoreLookInput _returnvalue false)
    (Input|SetInputModeGameOnly _returnvalue)))

(event Input|ActionEvents|InputActionTarget/UnTarget
  (params (Key :type Key%20Structure :default "None"))
  ;[1 1 1] Targeting
  (:Pressed
    (bind _foundtarget_ (CallFunction|ScanforTargets))
    (if _foundtarget_
      (CallFunction|ChooseTarget)
      (Default|CallTargetChanged)
      (else
        (CallFunction|LoseTarget)))))

(event Input|ActionEvents|InputActionBasic_Attack
  (params (Key :type Key%20Structure :default "None"))
  (bind _returnvalue (Game|GetPlayerCharacter 0))
  (:Pressed
    (Utilities|FlowControl|DoOnce false
      (:Completed
        (bind _returnvalue_2 (Game|SpawnActorfromClass "/Game/BluePrints/Skills/Monk/Attacks/Combo_Test_BP.Combo_Test_BP_C" (Math|Conversions|ToTransform(Vector) (Transformation|GetActorLocation _returnvalue)) "Undefined" 0 _returnvalue 0))))))

(event Input|ActionEvents|InputActionCancel_Attack
  (params (Key :type Key%20Structure :default "None"))
  (:Pressed
    (Default|CallInterruptCasting)
    (Animation|StopAnimMontage 0)
    (if (Utilities|IsValid (stale Input|ActionEvents|InputActionBasic_Attack _returnvalue_2))
      (Actor|DestroyActor (stale Input|ActionEvents|InputActionBasic_Attack _returnvalue_2))
      (CallFunction|UnlockComboEvent)
      (Variables|Default|SetAbilityComboCount 0)
      (Animation|PlayAnimMontage "/Game/Art_Assets/Animations/Monk/Block_Montage.Block_Montage" 1.0 "None")
      (elif (Game|Player|IsInputKeyDown (Game|GetPlayerController 0) Key)
        (Animation|PlayAnimMontage "/Game/Art_Assets/Animations/Monk/Block_Montage.Block_Montage" 1.0 "None"))))
  (:Released
    (Animation|StopAnimMontage 0)
    (Variables|Default|SetAbilityComboCount 0)))

(event Input|ActionEvents|InputActionFree_Mouse
  (params (Key :type Key%20Structure :default "None"))
  (bind _returnvalue (Game|GetPlayerController 0))
  ;[1 1 1] Free the Mouse
  (:Pressed
    (Input|SetInputModeGameandUI _returnvalue 0 "LockAlways" false)
    (Variables|/Script/Engine.PlayerController|SetbShowMouseCursor _returnvalue true))
  (:Released
    (Utilities|FlowControl|Delay 0.1)
    (Input|SetInputModeGameOnly _returnvalue)
    (Variables|/Script/Engine.PlayerController|SetbShowMouseCursor _returnvalue false)))

(event Input|MouseEvents|LeftMouseButton
  (params (Key :type Key%20Structure :default "None"))
  ;[1 1 1] Emoting
  (:Pressed
    (if (Variables|Default|GetIsEmoteWheelOpen)
      (CallFunction|EmoteSelection)
      (Utilities|FlowControl|Delay 3.0)
      (Pawn|Components|CharacterMovement|SetMovementMode (Variables|Character|GetCharacterMovement) "MOVE_Walking" 0))))

(event Input|KeyboardEvents|8
  (params (Key :type Key%20Structure :default "None"))
  ;[1 1 1] Savign test
  (:Pressed
    (bind _returnvalue (SaveGame|CreateSaveGameObject "/Game/BluePrints/SaveGame/SaveGame_BP.SaveGame_BP_C"))
    (bind _output_get (Variables|Default|SetSaveGameRef _returnvalue))
    (bind _output_get_2 (Variables|Default|SetPlayerLocation (Transformation|GetActorLocation)))
    (Variables|/Game/BluePrints/SaveGame/SaveGame_BP.SaveGame_BP_C|SetPlayerLocation_SG _output_get _output_get_2)
    (SaveGame|SaveGametoSlot _returnvalue "Test")
    (Development|PrintString "GameSaved")))

(event Input|KeyboardEvents|9
  (params (Key :type Key%20Structure :default "None"))
  ;[1 1 1] Savign test
  (:Pressed
    (bind _returnvalue (SaveGame|DoesSaveGameExist "Test"))
    (if _returnvalue
      (bind _returnvalue_2 (SaveGame|LoadGamefromSlot "Test"))
      (bind _assave_game_bp (Utilities|Casting|CastToSaveGame_BP _returnvalue_2))
      (bind _output_get (Variables|Default|SetPlayerLocation (Variables|/Game/BluePrints/SaveGame/SaveGame_BP.SaveGame_BP_C|GetPlayerLocation_SG _assave_game_bp)))
      (Transformation|SetActorLocation _output_get false false)
      (Development|PrintString "Hello")
      (else
        (Development|PrintString "Fuck off")))))

(fn ConstructionScript)

(fn ScanforTargets
  (bind _cameraboom (Variables|Default|GetCameraBoom))
  (bind _followcamera (Variables|Default|GetFollowCamera))
  (bind _returnvalue (Transformation|GetWorldLocation _cameraboom))
  (bind _returnvalue_2 (Transformation|GetWorldRotation _followcamera))
  (Utilities|Array|Clear (Variables|Default|GetCurrentTargetList))
  (bind _outhits (Collision|MultiSphereTraceForObjects _returnvalue (+ _returnvalue (* (Math|Vector|GetForwardVector (Math|Rotator|MakeRotator (.roll _returnvalue_2) 0.0 (.yaw _returnvalue_2))) 6e+02)) (LocalVariables|GetTargetingRange) (Utilities|Array|MakeArray "ObjectTypeQuery1" "ObjectTypeQuery2" "ObjectTypeQuery3") false 0 "ForDuration"))
  (for _array_element _outhits
    (if (Utilities|DoesObjectImplementInterface (.hitactor _array_element) "/Game/BluePrints/TargetingSystem/Targeting_Interface.Targeting_Interface_C")
      (Utilities|Array|AddUnique (LocalVariables|GetTargetList) (.hitactor _array_element))))
  (bind _output_get (Variables|Default|SetCurrentTargetList (LocalVariables|GetTargetList)))
  (return (> (Utilities|Array|Length _output_get) 0)))

(fn ChooseTarget
  (bind _currenttargetlist (Variables|Default|GetCurrentTargetList))
  (bind _output (Utilities|Array|Get(acopy) _currenttargetlist))
  (for _array_element _currenttargetlist
    (Rendering|SetVisibility (Actor|GetComponentsbyTag _array_element "/Script/UMG.WidgetComponent" "TargetIndicator") false false))
  (if (== (Variables|Default|GetCurrentTarget) _output)
    (CallFunction|LoseTarget)
    (else
      (bind _output_get (Variables|Default|SetCurrentTarget _output))
      (Rendering|SetVisibility (Actor|GetComponentsbyTag _output_get "/Script/UMG.WidgetComponent" "TargetIndicator") true false)
      (Rendering|SetVisibility (Actor|GetComponentsbyTag _output_get "/Script/UMG.WidgetComponent" "HealthBar") true false)
      (Variables|/Script/Engine.CharacterMovementComponent|SetMaxWalkSpeed (Variables|Character|GetCharacterMovement) 4e+02)
      (Variables|Default|SetLockedOnATarget true)
      (Rendering|SetVisibility (Variables|Default|GetSK_Blade) true false))))

(fn LookatTarget
  (bind _returnvalue (Game|GetPlayerController 0))
  (bind _returnvalue_2 (Pawn|GetControlRotation _returnvalue :!class /Script/Engine.Controller))
  (bind _currenttarget (Variables|Default|GetCurrentTarget)
    (:then
      (Transformation|SetActorRotation (Math|Rotator|MakeRotfromX (Math|Vector|GetUnitDirection(Vector) (Transformation|GetActorLocation) (Transformation|GetActorLocation _currenttarget))))
      (Pawn|SetControlRotation _returnvalue (Math|Rotator|MakeRotator (.Roll (Math|Rotator|BreakRotator (Math|Rotator|MakeRotfromX (Math|Vector|GetUnitDirection(Vector) (Transformation|GetActorLocation) (Transformation|GetActorLocation _currenttarget))))) (.pitch _returnvalue_2) (.yaw _returnvalue_2))))
    (:else)))

(fn LoseTarget
  (bind _currenttarget (Variables|Default|GetCurrentTarget)
    (:then
      (Rendering|SetVisibility (Actor|GetComponentsbyTag _currenttarget "/Script/UMG.WidgetComponent" "TargetIndicator") false false)
      (Rendering|SetVisibility (Actor|GetComponentsbyTag _currenttarget "/Script/UMG.WidgetComponent" "HealthBar") false false)
      (Variables|Default|SetCurrentTarget 0)
      (Utilities|Array|Clear (Variables|Default|GetCurrentTargetList))
      (Variables|/Script/Engine.CharacterMovementComponent|SetMaxWalkSpeed (Variables|Character|GetCharacterMovement) 6e+02)
      (Variables|Default|SetLockedOnATarget false)
      (Rendering|SetVisibility (Variables|Default|GetSK_Blade) false false))
    (:else)))

(fn PlayHighPrivorityMontage
  (params (Montage :type Anim%20Montage%20Object%20Reference) (InPlayRate :type Float%20%28single-precision%29) (StartSectionName :type Name))
  (if (not (Animation|Montage|MontageIsPlaying (Components|SkeletalMesh|GetAnimInstance (Variables|Character|GetMesh)) Montage))
    (bind _output_get (Variables|Default|SetHighPriorityMontage Montage))
    (bind _returnvalue (Animation|PlayAnimMontage _output_get InPlayRate StartSectionName))
    (return _returnvalue)))

(fn TryPlayMontage
  (params (Montage :type Anim%20Montage%20Object%20Reference) (InPlayRate :type Float%20%28single-precision%29) (StartSectionName :type Name))
  (if (not (Animation|Montage|MontageIsPlaying (Components|SkeletalMesh|GetAnimInstance (Variables|Character|GetMesh)) 0))
    (bind _returnvalue (Animation|PlayAnimMontage Montage InPlayRate StartSectionName))
    (return _returnvalue)))

(fn EmoteSelection
  (bind (_t _lt _rt _lb _rb _b) (Default|CallSelection (Variables|Default|GetEmoteWheelRef)))
  (if _t
    (Animation|PlayAnimMontage "/Game/Art_Assets/Animations/Emotes/Dance_Emote_1_Montage.Dance_Emote_1_Montage" 1.0 "None")
    (elif _lt
      (Animation|PlayAnimMontage "/Game/Art_Assets/Animations/Emotes/Angry_Sulk_Montage.Angry_Sulk_Montage" 1.0 "None")
      (elif _rt
        (Animation|PlayAnimMontage "/Game/Art_Assets/Animations/Emotes/Waving_Montage.Waving_Montage" 1.0 "None")
        (elif _lb
          (Animation|PlayAnimMontage "/Game/Art_Assets/Animations/Emotes/Stop_Agressive_Montage.Stop_Agressive_Montage" 1.0 "None")
          (elif _rb
            (Animation|PlayAnimMontage "/Game/Art_Assets/Animations/Emotes/Stop_Passive_Montage.Stop_Passive_Montage" 1.0 "None")
            (elif _b
              (Animation|PlayAnimMontage "/Game/Art_Assets/Animations/Emotes/Pointing_Montage.Pointing_Montage" 1.0 "None")
              (else
                (return))))))))
  (Pawn|Components|CharacterMovement|SetMovementMode (Variables|Character|GetCharacterMovement) "MOVE_None" 0)
  (Audio|PlaySoundatLocation "/Game/Art_Assets/Sounds/Terminated.Terminated" (Variables|Default|GetPlayerLocation) "0, 0, 0" 1.0 1.0 0.0 0 0 0))